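; Football actor for what appears to be a penalty shootout, launched by either a player shot or an AI shot.
; Shoot and ShootAI wait a given time, then apply a velocity-change impulse toward left, center or right, each using its own speed variable.
; Both start CheckIfGoal, which after a fixed delay reports a block to footBallGameMode and calls Alternate unless IsGoaled is set.
; The box overlap event is empty.
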(event `self.Box.OnComponentBeginOverlap`
  (params (OverlappedComponent :type "PrimitiveComponent Object Reference") (OtherActor :type "Actor Object Reference") (OtherComp :type "PrimitiveComponent Object Reference") (OtherBodyIndex :type Integer) (bFromSweep :type Boolean) (SweepResult :type "HitResult Structure (by ref)"))
  ;[1 1 1] on ball begin overlap
)

(event `shoot`
  (params (direction :type Integer) (time :type "Float (double-precision)"))
  (bind _football_speed (`self.football speed`))
  ;[1 1 1] shoot
  (set `self.started` true)
  (`KismetSystemLibrary.Delay` time)
  (`KismetSystemLibrary.PrintString` (`KismetStringLibrary.Concat_StrStr` "direction is " (`KismetStringLibrary.Conv_IntToString` direction)))
  (`self.checkIfGoal`)
  (`KismetSystemLibrary.PrintString` (`KismetStringLibrary.Conv_DoubleToString` _football_speed))
  (switch `int` direction
    (:`0`
      ;;[1 1 1] left
      (`PrimitiveComponent.AddImpulse` (`self.StaticMesh`) (* (2.0 -0.28 -0.185) _football_speed) "None" true))
    (:`1`
      ;;[1 1 1] center
      (`PrimitiveComponent.AddImpulse` (`self.StaticMesh`) (* (1.0 0.0 0.0) _football_speed) "None" true))
    (:`2`
      ;;[1 1 1] right
      (`PrimitiveComponent.AddImpulse` (`self.StaticMesh`) (* (0.878 0.436 -0.196) _football_speed) "None" true))))

(event `checkIfGoal`
  ;[1 1 1] check if goal
  (`KismetSystemLibrary.Delay` 4.0)
  (if (not (`self.isGoaled`))
    (bind _asfoot_ball_game_mode (cast `/Game/blueprints/footballgameMode/footBallGameMode` (`GameplayStatics.GetGameMode`)))
    (`/Game/blueprints/footballgameMode/footBallGameMode.onBlocked` _asfoot_ball_game_mode)
    (`/Game/blueprints/footballgameMode/footBallGameMode.alternate` _asfoot_ball_game_mode)))

(event `Key|LeftMouseButton`
  (params (Key :type "Key Structure")))

(event `ShootAI`
  (params (direction :type Integer) (time :type "Float (double-precision)"))
  (bind _footballsai_speed (`self.footballSAI speed`))
  ;[1 1 1] shoot AI
  (set `self.started` true)
  (`KismetSystemLibrary.Delay` time)
  (`KismetSystemLibrary.PrintString` (`KismetStringLibrary.Concat_StrStr` "direction is " (`KismetStringLibrary.Conv_IntToString` direction)))
  (`self.checkIfGoal`)
  (`KismetSystemLibrary.PrintString` (`KismetStringLibrary.Conv_DoubleToString` _footballsai_speed))
  (switch `int` direction
    (:`0`
      ;;[1 1 1] left
      (`PrimitiveComponent.AddImpulse` (`self.StaticMesh`) (* (2.2 -0.28 -0.185) _footballsai_speed) "None" true))
    (:`1`
      ;;[1 1 1] center
      (`PrimitiveComponent.AddImpulse` (`self.StaticMesh`) (* (1.0 0.0 0.0) _footballsai_speed) "None" true))
    (:`2`
      ;;[1 1 1] right
      (`PrimitiveComponent.AddImpulse` (`self.StaticMesh`) (* (0.878 0.2 -0.196) _footballsai_speed) "None" true))))

(fn `UserConstructionScript`)