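; Game mode for a football penalty shootout in which the player and AI alternate as kicker and goalkeeper.
; Tagged PlayerStarts set spawn transforms; each round respawns the ball and AI opponent, has the player controller spawn its role, then flips the turn.
; Goal, block and miss events trigger reactions and widgets, awarding points to the scorer or defender.
; Goals and misses also check for a winner at five points, which stops respawning.
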(event `self.ReceiveBeginPlay`
  ;[1 1 1] begin play
  (`KismetSystemLibrary.Delay` 0.2)
  (bind _outactors (`GameplayStatics.GetAllActorsOfClassWithTag` "/Script/Engine.PlayerStart" "goalKeeper"))
  (set `self.goalKeeperLoc` (`self.GetTransform` (`|GetArrayItem` _outactors)))
  (bind _outactors_2 (`GameplayStatics.GetAllActorsOfClassWithTag` "/Script/Engine.PlayerStart" "goalkicker"))
  (set `self.goalKickerLoc` (`self.GetTransform` (`|GetArrayItem` _outactors_2)))
  (bind _outactors_3 (`GameplayStatics.GetAllActorsOfClassWithTag` "/Script/Engine.PlayerStart" "footballPOs"))
  (set `self.footBallLoc` (`self.GetTransform` (`|GetArrayItem` _outactors_3)))
  (`self.spawnPlayerAndAI`))

(event `spawnPlayerAndAI`
  (bind _as_football_pc (`self.As Football PC`))
  ;[1 1 1] spawn player and goal keeper
  (if (not (`self.gameOver`))
    (`self.destroyIfValid` (`self.AIgoalKickerRef`))
    (`self.destroyIfValid` (`self.AiGoalkeeperRef`))
    (`self.destroyIfValid` (`self.football`))
    (if (`self.playerShouldKick`)
      (`/Game/blueprints/footballgameMode/footballPC.spawn Kicker` _as_football_pc)
      (bind _returnvalue (`|SpawnActorFromClass` "/Game/blueprints/characters/ai/aigoalKeeperActor.aigoalKeeperActor_C" (`self.goalKeeperLoc`) "AdjustIfPossibleButAlwaysSpawn" "OverrideRootScale" null null))
      (set `self.AiGoalkeeperRef` _returnvalue)
      (else
        (`/Game/blueprints/footballgameMode/footballPC.spawnGoalKeeper` _as_football_pc)
        (bind _returnvalue_2 (`|SpawnActorFromClass` "/Game/blueprints/characters/humans/AiNewgoalKicker.AiNewgoalKicker_C" (`self.goalKickerLoc`) "AdjustIfPossibleButAlwaysSpawn" "OverrideRootScale" null null))
        (set `self.AIgoalKickerRef` _returnvalue_2)))
    (bind _returnvalue_3 (`|SpawnActorFromClass` "/Game/blueprints/football/football.football_C" (`self.footBallLoc`) "AlwaysSpawn" "OverrideRootScale" null null))
    (set `self.football` _returnvalue_3)
    (set `self.playerShouldKick` (not (`self.playerShouldKick`)))))

(event `self.K2_PostLogin`
  (params (NewPlayer :type "PlayerController Object Reference"))
  ;[1 1 1] event on post login
  (bind _asfootball_pc (cast `/Game/blueprints/footballgameMode/footballPC` NewPlayer))
  (set `self.As Football PC` _asfootball_pc))

(event `alternate`
  ;[1 1 1] alternate
  (`KismetSystemLibrary.Delay` 3.0)
  (`self.spawnPlayerAndAI`))

(event `notKicked`
  (bind _aigoalkeeperref (`self.AiGoalkeeperRef`))
  ;[1 1 1] on not kicked
  (`/Engine/EditorBlueprintResources/StandardMacros.IsValid` _aigoalkeeperref
    (:`Is Valid`
      (bind _outactors (`GameplayStatics.GetAllActorsOfClass` "/Game/blueprints/characters/humans/goalKicker_Child.goalKicker_Child_C"))
      (`/Game/blueprints/characters/humans/goalKicker_Child.sad` (`|GetArrayItem` _outactors))
      (`/Game/blueprints/characters/ai/aigoalKeeperActor.celebrate` _aigoalkeeperref))
    (:`Is Not Valid`
      (`/Game/blueprints/characters/humans/goalKicker_Child.sad` (`self.AIgoalKickerRef`))
      (bind _outactors_2 (`GameplayStatics.GetAllActorsOfClass` "/Game/blueprints/characters/humans/HumangoalKeeperActor.HumangoalKeeperActor_C"))
      (`/Game/blueprints/characters/humans/HumangoalKeeperActor.celebrate` (`|GetArrayItem` _outactors_2))))
  (bind _returnvalue (`|CreateWidget` "/Game/blueprints/UI/onMissed.onMissed_C"))
  (`UserWidget.AddToViewport` _returnvalue 0)
  (if (`self.playerShouldKick`)
    (`/Engine/EditorBlueprintResources/StandardMacros.IncrementInt` (`self.playerScore`)
      (:`  `
        (`self.checkIfWon`)))
    (else
      (`/Engine/EditorBlueprintResources/StandardMacros.IncrementInt` (`self.aiScore`)
        (:`  `
          (`self.checkIfWon`)))))
  (`KismetSystemLibrary.Delay` 2.0)
  (`self.alternate`))

(event `onGoal`
  (bind _aigoalkeeperref (`self.AiGoalkeeperRef`))
  ;[1 1 1] on goal
  (`KismetSystemLibrary.PrintString` "Hello")
  (`/Engine/EditorBlueprintResources/StandardMacros.IsValid` _aigoalkeeperref
    (:`Is Valid`
      (bind _outactors (`GameplayStatics.GetAllActorsOfClass` "/Game/blueprints/characters/humans/goalKicker_Child.goalKicker_Child_C"))
      (`/Game/blueprints/characters/humans/goalKicker.celebrate` (`|GetArrayItem` _outactors))
      (`/Game/blueprints/characters/ai/aigoalKeeperActor.sad` _aigoalkeeperref))
    (:`Is Not Valid`
      (`/Game/blueprints/characters/humans/goalKicker.celebrate` (`self.AIgoalKickerRef`))
      (bind _outactors_2 (`GameplayStatics.GetAllActorsOfClass` "/Game/blueprints/characters/humans/HumangoalKeeperActor.HumangoalKeeperActor_C"))
      (`/Game/blueprints/characters/humans/HumangoalKeeperActor.sad` (`|GetArrayItem` _outactors_2))))
  (bind _returnvalue (`|CreateWidget` "/Game/blueprints/UI/onGoal.onGoal_C"))
  (`UserWidget.AddToViewport` _returnvalue 0)
  (if (`self.playerShouldKick`)
    (`/Engine/EditorBlueprintResources/StandardMacros.IncrementInt` (`self.aiScore`)
      (:`  `
        (`self.checkIfWon`)))
    (else
      (`/Engine/EditorBlueprintResources/StandardMacros.IncrementInt` (`self.playerScore`)
        (:`  `
          (`self.checkIfWon`))))))

(event `onBlocked`
  (bind _aigoalkeeperref (`self.AiGoalkeeperRef`))
  ;[1 1 1] on blocked
  (`/Engine/EditorBlueprintResources/StandardMacros.IsValid` _aigoalkeeperref
    (:`Is Valid`
      (bind _outactors (`GameplayStatics.GetAllActorsOfClass` "/Game/blueprints/characters/humans/goalKicker_Child.goalKicker_Child_C"))
      (`/Game/blueprints/characters/humans/goalKicker_Child.sad` (`|GetArrayItem` _outactors))
      (`/Game/blueprints/characters/ai/aigoalKeeperActor.celebrate` _aigoalkeeperref))
    (:`Is Not Valid`
      (`/Game/blueprints/characters/humans/goalKicker_Child.sad` (`self.AIgoalKickerRef`))
      (bind _outactors_2 (`GameplayStatics.GetAllActorsOfClass` "/Game/blueprints/characters/humans/HumangoalKeeperActor.HumangoalKeeperActor_C"))
      (`/Game/blueprints/characters/humans/HumangoalKeeperActor.celebrate` (`|GetArrayItem` _outactors_2))))
  (bind _returnvalue (`|CreateWidget` "/Game/blueprints/UI/onBlocked.onBlocked_C"))
  (`UserWidget.AddToViewport` _returnvalue 0)
  (if (`self.playerShouldKick`)
    (`/Engine/EditorBlueprintResources/StandardMacros.IncrementInt` (`self.playerScore`))
    (else
      (`/Engine/EditorBlueprintResources/StandardMacros.IncrementInt` (`self.aiScore`)))))

(event `checkIfWon`
  ;[1 1 1] check if won
  (if (>= (`self.aiScore`) 5)
    (if (!= (`self.aiScore`) (`self.playerScore`))
      (set `self.gameOver` true)
      (bind _returnvalue (`|CreateWidget` "/Game/blueprints/UI/AIWon.AIWon_C"))
      (`UserWidget.AddToViewport` _returnvalue 0))
    (elif (>= (`self.playerScore`) 5)
      (set `self.gameOver` true)
      (bind _returnvalue_2 (`|CreateWidget` "/Game/blueprints/UI/playerWon.playerWon_C"))
      (`UserWidget.AddToViewport` _returnvalue_2 0))))

(fn `destroyIfValid`
  (params (NewParam :type "Actor Object Reference"))
  (`/Engine/EditorBlueprintResources/StandardMacros.IsValid` NewParam
    (:`Is Valid`
      (`self.K2_DestroyActor` NewParam))))

(fn `UserConstructionScript`)