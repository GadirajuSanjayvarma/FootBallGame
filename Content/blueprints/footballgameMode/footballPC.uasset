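; Football player controller that switches between goal kicker and goalkeeper roles, spawning each at tagged PlayerStarts.
; It creates the UI, feeds movement axes to an on-screen image and toggles the UI per role.
; Each spawn destroys the other role's actor; the kicker spawn also switches view to the first CameraActor.
; Screen positions are deprojected into debug line traces from the kicker that only print the hit actor.
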(event `self.ReceiveBeginPlay`
  ;[1 1 1] begin play
  (bind _outactors (`GameplayStatics.GetAllActorsOfClassWithTag` "/Script/Engine.PlayerStart" "goalKeeper"))
  (set `self.goalKeeperLoc` (`self.GetTransform` (`|GetArrayItem` _outactors)))
  (bind _outactors_2 (`GameplayStatics.GetAllActorsOfClassWithTag` "/Script/Engine.PlayerStart" "goalkicker"))
  (set `self.goalKickerLoc` (`self.GetTransform` (`|GetArrayItem` _outactors_2)))
  (bind _returnvalue (`|CreateWidget` "/Game/blueprints/UI/userInterface.userInterface_C"))
  (`UserWidget.AddToViewport` _returnvalue 0)
  (set `self.UI` _returnvalue)
  (set `/Game/blueprints/UI/userInterface.footballPC` self _returnvalue))

(event `InputAxis|MoveForward`
  (params (AxisValue :type "Float (single-precision)"))
  (set `self.forwardVal` AxisValue)
  (`/Game/blueprints/UI/userInterface.updateImgPos` (`self.UI`) (`KismetMathLibrary.MakeVector2D` (* (`self.forwardVal`) 10.0) (* (`self.rightVal`) 10.0))))

(event `InputAxis|MoveRight`
  (params (AxisValue :type "Float (single-precision)"))
  (set `self.rightVal` AxisValue)
  (`/Game/blueprints/UI/userInterface.updateImgPos` (`self.UI`) (`KismetMathLibrary.MakeVector2D` (* (`self.forwardVal`) 10.0) (* (`self.rightVal`) 10.0))))

(event `spawn Kicker`
  ;[1 1 1] spawn kicker
  (`/Game/blueprints/UI/userInterface.enable/Disable` (`self.UI`) true)
  (`self.destroyIfValid` (`self.Goalkeeper Ref`))
  (bind _returnvalue (`|SpawnActorFromClass` "/Game/blueprints/characters/humans/goalKicker_Child.goalKicker_Child_C" (`self.goalKickerLoc`) "AlwaysSpawn" "OverrideRootScale" null null))
  (bind _output_get (set `self.goal Kicker Ref` _returnvalue))
  (bind _outactors (`GameplayStatics.GetAllActorsOfClass` "/Script/Engine.CameraActor"))
  (bind _output (`|GetArrayItem` _outactors))
  (set `self.cameraVar` _output)
  (`self.SetViewTargetWithBlend` _output))

(event `spawnGoalKeeper`
  ;[1 1 1] spawn goal keeper
  (`/Game/blueprints/UI/userInterface.enable/Disable` (`self.UI`) false)
  (`self.destroyIfValid` (`self.goal Kicker Ref`))
  (bind _returnvalue (`|SpawnActorFromClass` "/Game/blueprints/characters/humans/HumangoalKeeperActor.HumangoalKeeperActor_C" (`self.goalKeeperLoc`) "AdjustIfPossibleButAlwaysSpawn" "OverrideRootScale" null null))
  (set `self.Goalkeeper Ref` _returnvalue))

(event `castRay`
  (params (endPos :type "Vector Structure"))
  ;[1 1 1] tocuh
  (`/Engine/EditorBlueprintResources/StandardMacros.IsValid` (`self.goal Kicker Ref`)
    (:`Is Valid`
      (`KismetSystemLibrary.PrintString` "doing screen cast")
      (bind _outhit (`KismetSystemLibrary.LineTraceSingle` (`self.K2_GetActorLocation` (`self.goal Kicker Ref`)) (* endPos 10000.0) "TraceTypeQuery1" false (`|MakeArray` self :!type "Actor Object Reference") "Persistent"))
      (`KismetSystemLibrary.PrintString` (`KismetSystemLibrary.GetDisplayName` (`.HitActor` (`GameplayStatics.BreakHitResult` _outhit)))))))

(event `toWorld`
  (params (pos :type "Vector2D Structure"))
  ;[1 1 1] to world cast
  (`self.castRay` (`GameplayStatics.DeprojectScreenToWorld` self pos)))

(fn `destroyIfValid`
  (params (NewParam :type "Actor Object Reference"))
  (`/Engine/EditorBlueprintResources/StandardMacros.IsValid` NewParam
    (:`Is Valid`
      (`self.K2_DestroyActor` NewParam))))

(fn `UserConstructionScript`)